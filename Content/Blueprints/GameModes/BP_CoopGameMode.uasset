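; Co-op game mode that adds a second local player on BeginPlay.
; It creates a player with an automatic controller ID, spawns BP_OtherSamurai at the "Player2" player start and possesses it with the new controller.
; A matching BP_RedSamurai setup for "Player1" is left unconnected and never runs, and Tick is unused.
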(event `self.ReceiveBeginPlay`
  (`|ExecutionSequence`
    (:`then_1`
      (bind _returnvalue (`GameplayStatics.CreatePlayer` -1))
      (bind _returnvalue_2 (`|SpawnActorFromClass` "/Game/Blueprints/Characters/BP_OtherSamurai.BP_OtherSamurai_C" (`KismetMathLibrary.MakeTransform` (`self.K2_GetActorLocation` (`self.K2_FindPlayerStart` _returnvalue "Player2"))) "Undefined" "MultiplyWithRoot" null null))
      (`Controller.Possess` _returnvalue _returnvalue_2))))

(fn `UserConstructionScript`)